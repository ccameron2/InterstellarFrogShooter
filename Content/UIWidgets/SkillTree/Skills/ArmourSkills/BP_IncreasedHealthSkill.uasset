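; Armour skill tree Blueprint that raises the player's health when applied.
; ApplySkill runs the parent logic, then, if the skill tree component is valid, increments its armour skill count.
; It casts the owner to the main player controller and its pawn to the player character, then adds a fixed bonus to both current and maximum health.
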(fn ApplySkill
  (params (Owner :type Actor%20Object%20Reference))
  (bind _skilltreecomponent (Variables|Default|GetskillTreeComponent))
  (|CallParentFunction Owner)
  (Utilities|IsValid _skilltreecomponent
    (:Is%20Valid
      (Math|Integer|IncrementInt (Variables|/Game/UIWidgets/SkillTree/SkillTreeComponent.SkillTreeComponent_C|GetCurrentArmourSkillCount _skilltreecomponent)
        (:%20%20
          (bind _asbp_main_player_controller (Utilities|Casting|CastToBP_MainPlayerController Owner))
          (bind _asbp_player_character (Utilities|Casting|CastToBP_PlayerCharacter (Pawn|GetControlledPawn _asbp_main_player_controller)))
          (Variables|/Script/TeamProject.PlayerCharacter|SetPlayerHealth _asbp_player_character (+ (Variables|/Script/TeamProject.PlayerCharacter|GetPlayerHealth _asbp_player_character) 5e+01))
          (Variables|/Script/TeamProject.PlayerCharacter|SetPlayerMaxHealth _asbp_player_character (+ (Variables|/Script/TeamProject.PlayerCharacter|GetPlayerMaxHealth _asbp_player_character) 50)))))))