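; Drone skill tree skill that unlocks the minimap and spawns a drone for the player.
; ApplySkill runs the parent logic, then, if the skill tree component is valid, increments the acquired drone skill count.
; It then casts the owner to the player controller and its controlled pawn to the player character, calling UnlockMiniMap on the LevelComponent and SpawnDrone on the character.
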(fn ApplySkill
  (params (Owner :type Actor%20Object%20Reference))
  (bind _skilltreecomponent (Variables|Default|GetskillTreeComponent))
  ;[1 1 1] Check if the SkillTreeComponent Exists and increment the amount of skills Acquired in the current branch
  (|CallParentFunction Owner)
  (Utilities|IsValid _skilltreecomponent
    (:Is%20Valid
      (Math|Integer|IncrementInt (Variables|/Game/UIWidgets/SkillTree/SkillTreeComponent.SkillTreeComponent_C|GetCurrentDroneSkillCount _skilltreecomponent)
        (:%20%20
          ;[1 1 1] Unlock a Drone and spawn it in the game and Unlock the MiniMap for the Player
          (bind _asbp_main_player_controller (Utilities|Casting|CastToBP_MainPlayerController Owner))
          (bind _asbp_player_character (Utilities|Casting|CastToBP_PlayerCharacter (Pawn|GetControlledPawn _asbp_main_player_controller)))
          (Class|LevellingUpComponent|UnlockMiniMap (Variables|/Script/TeamProject.PlayerCharacter|GetLevelComponent _asbp_player_character))
          (Class|PlayerCharacter|SpawnDrone _asbp_player_character))))))