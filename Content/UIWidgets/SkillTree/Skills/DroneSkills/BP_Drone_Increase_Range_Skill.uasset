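; Skill-tree skill that boosts the attack range of the player's drone when applied.
; ApplySkill runs the parent logic, then, if the SkillTreeComponent is valid, increments the drone branch's acquired-skill count.
; It then casts from the owning player controller through the pawn to its drone and multiplies AttackRange by 1.5.
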(fn ApplySkill
  (params (Owner :type Actor%20Object%20Reference))
  (bind _skilltreecomponent (Variables|Default|GetskillTreeComponent))
  ;[1 1 1] Check if the SkillTreeComponent Exists and increment the amount of skills Acquired in the current branch
  (|CallParentFunction Owner)
  (Utilities|IsValid _skilltreecomponent
    (:Is%20Valid
      (Math|Integer|IncrementInt (Variables|/Game/UIWidgets/SkillTree/SkillTreeComponent.SkillTreeComponent_C|GetCurrentDroneSkillCount _skilltreecomponent)
        (:%20%20
          ;[1 1 1] Increase the Drones Range through the Drones Blueprint
          ;  - currently increases the Drones Range by 1.5x
          (bind _asbp_main_player_controller (Utilities|Casting|CastToBP_MainPlayerController Owner))
          (bind _asbp_player_character (Utilities|Casting|CastToBP_PlayerCharacter (Pawn|GetControlledPawn _asbp_main_player_controller)))
          (bind _asbp_drone (Utilities|Casting|CastToBP_Drone (Class|PlayerCharacter|GetDrone _asbp_player_character)))
          (Variables|/Script/TeamProject.Drone|SetAttackRange _asbp_drone (* (Variables|/Script/TeamProject.Drone|GetAttackRange _asbp_drone) 1.5)))))))