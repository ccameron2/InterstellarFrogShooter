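; BP_Skill is the base Blueprint for a skill tree skill, holding its category and status.
; ApplySkill, extended by child skills, casts the owner to BP_MainPlayerController, caches its SkillTreeComponent and marks the skill Acquired.
; RequestAcquire fires the OnAquireRequest dispatcher with the category and itself, so purchases are handed to listeners rather than applied directly.
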(fn GetStatus
  ;[1 1 1] Get the status of the Skill
  (return (Variables|Default|GetStatus)))

(fn SetStatus
  (params (Status :type E_SkillStatus%20Enum :default "NewEnumerator0"))
  ;[1 1 1] Set the status of the Skill
  (Variables|Default|SetStatus Status))

(fn ApplySkill
  (params (Owner :type Actor%20Object%20Reference))
  ;[1 1 1] Update the Status to be 'Acquired', This function is called on the chosen child class as well
  (bind _asbp_main_player_controller (Utilities|Casting|CastToBP_MainPlayerController Owner))
  (Variables|Default|SetskillTreeComponent (Variables|/Game/Blueprints/BP_MainPlayerController.BP_MainPlayerController_C|GetSkillTreeComponent _asbp_main_player_controller))
  (Variables|Default|SetStatus "NewEnumerator2"))

(fn RequestAcquire
  ;[1 1 1] Call the 'OnSkillAcquired' function in the SkillTreeComponent when this skill is purchased
  (Default|CallOnAquireRequest (Variables|Default|GetCategory) self))