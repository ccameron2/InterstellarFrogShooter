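; Player controller for the main player, handling menu hotkeys and a key that grants XP.
; The SkillTree action toggles between two screens through WidgetLoader, restoring game-only input and hiding the cursor on close.
; P loads another widget with UI-only input and a visible cursor.
; L adds a fixed amount of XP through the player character's LevelComponent.
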(event EventBeginPlay)

(event EventTick
  (params (DeltaSeconds :type Float%20%28single-precision%29)))

(event Input|ActionEvents|InputActionSkillTree
  (params (Key :type Key%20Structure :default "None"))
  (bind _self self)
  (:Pressed
    (bind _output_get (Variables|Default|SetSkillTreeOpen (not (Variables|Default|GetSkillTreeOpen))))
    (if _output_get
      (Class|MainPlayerController|WidgetLoader _self 3)
      (else
        (Class|MainPlayerController|WidgetLoader _self 1)
        (Input|SetInputModeGameOnly _self false)
        (Variables|/Script/Engine.PlayerController|SetbShowMouseCursor _self false)))))

(event Input|KeyboardEvents|P
  (params (Key :type Key%20Structure :default "None"))
  (bind _self self)
  (:Pressed
    (Class|MainPlayerController|WidgetLoader _self 4)
    (Input|SetInputModeUIOnly _self 0 "DoNotLock" false)
    (Variables|/Script/Engine.PlayerController|SetbShowMouseCursor _self true)))

(event Input|KeyboardEvents|L
  (params (Key :type Key%20Structure :default "None"))
  (:Pressed
    (bind _asbp_player_character (Utilities|Casting|CastToBP_PlayerCharacter (Game|GetPlayerCharacter 0)))
    (Class|LevellingUpComponent|AddXP (Variables|/Script/TeamProject.PlayerCharacter|GetLevelComponent _asbp_player_character) 25.0)))

(fn ConstructionScript)