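; Player controller that sets up the mech skill tree and handles its menu input.
; On BeginPlay it constructs weapon, armour and drone skill objects in code, registers them per category with SkillTreeComponent, then creates the SkillTree widget from that component.
; The SkillTree action toggles the widget, switching input mode and cursor.
; P calls WidgetLoader in UI-only mode, and L grants the character XP through its LevelComponent.
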(event EventBeginPlay
  (CallFunction|InitSkills)
  (bind _returnvalue (UserInterface|CreateWidget "/Game/UIWidgets/SkillTree/SkillTree.SkillTree_C" self (Variables|Default|GetSkillTreeComponent)))
  (Variables|Default|SetSkillWidget _returnvalue))

(event EventTick
  (params (DeltaSeconds :type Float%20%28single-precision%29)))

(event Input|ActionEvents|InputActionSkillTree
  (params (Key :type Key%20Structure :default "None"))
  (bind _self self)
  (bind _skillwidget (Variables|Default|GetSkillWidget))
  (:Pressed
    (if (UserInterface|Viewport|IsinViewport _skillwidget)
      (Widget|RemovefromParent _skillwidget)
      (Input|SetInputModeGameOnly _self false)
      (Variables|Default|SetbShowMouseCursor false)
      (else
        (UserInterface|Viewport|AddtoViewport _skillwidget 0)
        (Input|SetInputModeGameandUI _self (Variables|Default|GetSkillWidget) "LockAlways" false false)
        (Variables|Default|SetbShowMouseCursor true)))))

(event Input|KeyboardEvents|P
  (params (Key :type Key%20Structure :default "None"))
  (bind _self self)
  (:Pressed
    (Class|MainPlayerController|WidgetLoader _self 4)
    (Input|SetInputModeUIOnly _self 0 "DoNotLock" false)
    (Variables|/Script/Engine.PlayerController|SetbShowMouseCursor _self true)))

(event Input|KeyboardEvents|L
  (params (Key :type Key%20Structure :default "None"))
  (:Pressed
    (bind _asbp_player_character (Utilities|Casting|CastToBP_PlayerCharacter (Game|GetPlayerCharacter 0)))
    (Class|LevellingUpComponent|AddXP (Variables|/Script/TeamProject.PlayerCharacter|GetLevelComponent _asbp_player_character) 25.0)))

(fn ConstructionScript)

(fn InitSkills
  (bind _self self)
  (Utilities|FlowControl|Sequence
    (:then_0
      (bind _returnvalue (Game|ConstructObjectfromClass _self "/Game/UIWidgets/SkillTree/Skills/WeaponSkills/BP_WeaponSkill_AquireNewWeapon.BP_WeaponSkill_AquireNewWeapon_C" (Variables|Default|GetWeaponCategory) "Energy Weapon" "Install an Energy weapon onto your mech" 0))
      (bind _returnvalue_2 (Game|ConstructObjectfromClass _self "/Game/UIWidgets/SkillTree/Skills/WeaponSkills/BP_WeaponSkill_DoubleDamage.BP_WeaponSkill_DoubleDamage_C" (Variables|Default|GetWeaponCategory) "Double Damage" "Get double your damage" "/Game/UIWidgets/SkillTextures/DamageMultiplier.DamageMultiplier"))
      (Default|AddSkillArray (Variables|Default|GetSkillTreeComponent) (Variables|Default|GetWeaponCategory) (Utilities|Array|MakeArray _returnvalue _returnvalue_2)))
    (:then_1
      (bind _returnvalue_3 (Game|ConstructObjectfromClass self "/Game/UIWidgets/SkillTree/Skills/ArmourSkills/BP_ArmourSkill.BP_ArmourSkill_C" (Variables|Default|GetArmourCategory) "Armour" "Add armour to your mech" 0))
      (bind _returnvalue_4 (Game|ConstructObjectfromClass self "/Game/UIWidgets/SkillTree/Skills/ArmourSkills/BP_ReducedDamageSkill.BP_ReducedDamageSkill_C" (Variables|Default|GetArmourCategory) "Reduced Damage" "Take reduced damage from enemies" 0))
      (bind _returnvalue_5 (Game|ConstructObjectfromClass self "/Game/UIWidgets/SkillTree/Skills/ArmourSkills/BP_DodgeChanceSkill.BP_DodgeChanceSkill_C" (Variables|Default|GetArmourCategory) "Dodge chance" "Add a chance to dodge enemy bullets" 0))
      (bind _returnvalue_6 (Game|ConstructObjectfromClass self "/Game/UIWidgets/SkillTree/Skills/ArmourSkills/BP_IncreasedHealthSkill.BP_IncreasedHealthSkill_C" (Variables|Default|GetArmourCategory) "Increased Health" "Increase your Mechs health" 0))
      (bind _returnvalue_7 (Game|ConstructObjectfromClass self "/Game/UIWidgets/SkillTree/Skills/ArmourSkills/BP_IncreasedDodgeChanceSkill.BP_IncreasedDodgeChanceSkill_C" (Variables|Default|GetArmourCategory) "Increased dodge chance" "Increase your dodge chance further" 0))
      (bind _returnvalue_8 (Game|ConstructObjectfromClass self "/Game/UIWidgets/SkillTree/Skills/ArmourSkills/BP_PassiveRegenSkill.BP_PassiveRegenSkill_C" (Variables|Default|GetArmourCategory) "Passive health regen" "Passively regenerate your Mechs health" 0))
      (bind _returnvalue_9 (Game|ConstructObjectfromClass self "/Game/UIWidgets/SkillTree/Skills/ArmourSkills/BP_EnergyShieldSkill.BP_EnergyShieldSkill_C" (Variables|Default|GetArmourCategory) "Energy Shield" "Add an Energy shield to your mech" 0))
      (Default|AddSkillArray (Variables|Default|GetSkillTreeComponent) (Variables|Default|GetArmourCategory) (Utilities|Array|MakeArray _returnvalue_3 _returnvalue_4 _returnvalue_5 _returnvalue_6 _returnvalue_7 _returnvalue_8 _returnvalue_9)))
    (:then_2
      (bind _returnvalue_10 (Game|ConstructObjectfromClass self "/Game/UIWidgets/SkillTree/Skills/DroneSkills/BP_DroneMiniMapSkill.BP_DroneMiniMapSkill_C" (Variables|Default|GetDroneCategory) "Drone + Minimap" "Gain access to a Drone and Minimap" 0))
      (bind _returnvalue_11 (Game|ConstructObjectfromClass self "/Game/UIWidgets/SkillTree/Skills/DroneSkills/BP_FasterFlightSkill.BP_FasterFlightSkill_C" (Variables|Default|GetDroneCategory) "Faster Flight" "Your drone is able to fly faster" 0))
      (bind _returnvalue_12 (Game|ConstructObjectfromClass self "/Game/UIWidgets/SkillTree/Skills/DroneSkills/BP_DroneGunSkill.BP_DroneGunSkill_C" (Variables|Default|GetDroneCategory) "Drone Gun" "Your drone now has access to a Gun" 0))
      (bind _returnvalue_13 (Game|ConstructObjectfromClass self "/Game/UIWidgets/SkillTree/Skills/DroneSkills/BP_ReducedCooldownSkill.BP_ReducedCooldownSkill_C" (Variables|Default|GetDroneCategory) "Reduced cooldown" "Reduce the cooldown of your drone" 0))
      (bind _returnvalue_14 (Game|ConstructObjectfromClass self "/Game/UIWidgets/SkillTree/Skills/DroneSkills/BP_EnergyBurnSkill.BP_EnergyBurnSkill_C" (Variables|Default|GetDroneCategory) "Drone Energy burn" "Your drone now has the ability to energy burn your enemies" 0))
      (bind _returnvalue_15 (Game|ConstructObjectfromClass self "/Game/UIWidgets/SkillTree/Skills/DroneSkills/BP_DronePlasmaSkill.BP_DronePlasmaSkill_C" (Variables|Default|GetDroneCategory) "Drone Plasma" "Your drone nowhasa plasma weapon" 0))
      (bind _returnvalue_16 (Game|ConstructObjectfromClass self "/Game/UIWidgets/SkillTree/Skills/DroneSkills/BP_LargerMiniMapSkill.BP_LargerMiniMapSkill_C" (Variables|Default|GetDroneCategory) "Increased Minimap range" "Increase the amount your minimap can see" 0))
      (Default|AddSkillArray (Variables|Default|GetSkillTreeComponent) (Variables|Default|GetDroneCategory) (Utilities|Array|MakeArray _returnvalue_10 _returnvalue_11 _returnvalue_12 _returnvalue_13 _returnvalue_14 _returnvalue_15 _returnvalue_16)))))